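; BP_Enemy_AI is an AI-controlled enemy Blueprint that passes combat state changes on to its AI blackboard.
; On BeginPlay it runs the parent logic and binds to the StateComponent's state-type-changed event.
; Entering the Hitted or Blocked state sets the Behavior enum key on its AI controller's blackboard to a value specific to that reaction.
; The construction script only calls the parent's.
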(event Custom|OnStateTypeChanged_AI
  (params (InPrevType :type EStateType%20Enum :default "NewEnumerator0") (InNewType :type EStateType%20Enum :default "NewEnumerator0"))
  (bind _returnvalue (Utilities|Name|MakeLiteralName "Behavior"))
  (bind _self self)
  (bind _returnvalue_2 (AI|GetAIController _self))
  (bind _returnvalue_3 (AI|GetBlackboard _returnvalue_2))
  (switch Utilities|FlowControl|Switch|SwitchonEStateType InNewType
    (:NewEnumerator5
      (AI|Components|Blackboard|SetValueasEnum _returnvalue_3 _returnvalue (Utilities|Enum|LiteralenumEBehaviorType "NewEnumerator4")))
    (:NewEnumerator8
      (AI|Components|Blackboard|SetValueasEnum _returnvalue_3 _returnvalue (Utilities|Enum|LiteralenumEBehaviorType "NewEnumerator6")))))

(event EventBeginPlay
  (|CallParentFunction)
  (EventDispatchers|BindEventtoOnStateTypeChanged (Variables|Default|GetStateComponent) (delegate Custom|OnStateTypeChanged_AI)))

(fn ConstructionScript
  (|CallParentFunction))