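; Boss area-of-effect skill actor that telegraphs a targeting circle, then becomes a burning damage field after a short delay.
; Player overlap spawns a post-process actor and a delayed burn emitter on the player's mesh, and sends unavoidable damage messages every Tick.
; Leaving the sphere clears these effects and stops damage after a delay, while EndPlay cleans up the field, post-process and burn effects.
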(event OnComponentBeginOverlap(Sphere)
  (params (OverlappedComponent :type Primitive%20Component%20Object%20Reference) (OtherActor :type Actor%20Object%20Reference) (OtherComp :type Primitive%20Component%20Object%20Reference) (OtherBodyIndex :type Integer) (bFromSweep :type Boolean) (SweepResult :type Hit%20Result%20Structure%20%28by%20ref%29))
  (if (== OtherActor (Game|GetPlayerCharacter 0))
    (Variables|Default|SetDamageOn true)
    (bind _returnvalue (Game|SpawnActorfromClass "/Game/Enemies/Boss/BP_BossPostProcess.BP_BossPostProcess_C" (Transformation|GetActorTransform) "Undefined" 0 0))
    (Variables|Default|SetPostProcess _returnvalue)
    (Utilities|FlowControl|Delay 1.0)
    (bind _returnvalue_2 (Effects|SpawnEmitterAttached "/Game/Effects/P_BossSkillBurn.P_BossSkillBurn" (Variables|/Script/Engine.Character|GetMesh (Game|GetPlayerCharacter 0)) "None" "0, 0, 0" "0, 0, 0" "0.600000,0.600000,1.000000"))
    (Variables|Default|SetP_Burn _returnvalue_2)))

(event OnComponentEndOverlap(Sphere)
  (params (OverlappedComponent :type Primitive%20Component%20Object%20Reference) (OtherActor :type Actor%20Object%20Reference) (OtherComp :type Primitive%20Component%20Object%20Reference) (OtherBodyIndex :type Integer))
  (bind _postprocess (Variables|Default|GetPostProcess))
  (bind _p_burn (Variables|Default|GetP_Burn))
  (if (== OtherActor (Game|GetPlayerCharacter 0))
    (Utilities|FlowControl|Delay 3.0)
    (Utilities|IsValid _postprocess
      (:Is%20Valid
        (Actor|DestroyActor _postprocess)
        (Utilities|IsValid _p_burn
          (:Is%20Valid
            (Components|Activation|Deactivate _p_burn)
            (Variables|Default|SetDamageOn false)))))))

(event EventBeginPlay
  (Collision|SetCollisionEnabled (Variables|Default|GetSphere) "NoCollision")
  (Utilities|FlowControl|Delay 3.0)
  (Components|DestroyComponent (Variables|Default|GetNS_Targeting_Circle))
  (Collision|SetCollisionEnabled (Variables|Default|GetSphere) "QueryAndPhysics")
  (bind _returnvalue (Effects|SpawnEmitteratLocation "/Game/Effects/P_DmgField_Fire_02.P_DmgField_Fire_02" (Transformation|GetActorLocation))))

(event EventEndPlay
  (params (EndPlayReason :type EEndPlayReason%20Enum :default "Destroyed"))
  (bind _postprocess (Variables|Default|GetPostProcess))
  (bind _p_burn (Variables|Default|GetP_Burn))
  (Utilities|IsValid (stale EventBeginPlay _returnvalue)
    (:Is%20Valid
      (Components|DestroyComponent (stale EventBeginPlay _returnvalue))
      (Utilities|IsValid _postprocess
        (:Is%20Valid
          (Actor|DestroyActor _postprocess)
          (Utilities|IsValid _p_burn
            (:Is%20Valid
              (Components|Activation|Deactivate _p_burn))))))))

(event EventTick
  (params (DeltaSeconds :type Float%20%28single-precision%29))
  (if (Variables|Default|GetDamageOn)
    (Class|IDamage|Damaged(Message) (Game|GetPlayerCharacter 0) 0 self (Variables|Default|GetHit%20Data) true)))

(fn ConstructionScript)