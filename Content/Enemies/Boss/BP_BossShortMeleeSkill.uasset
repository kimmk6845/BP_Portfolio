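; Boss short-range melee skill actor that launches as a moving, expanding damage sphere aimed at the player character.
; Activate sets the projectile movement velocity from a given direction and starts it, while Tick eases the sphere radius toward MaxRadius.
; Overlap events track whether the player is inside, and Tick sends DamagedMessage every frame while they are, with avoidance disabled and the player passed as Attacker.
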(event OnComponentBeginOverlap(Sphere)
  (params (OverlappedComponent :type Primitive%20Component%20Object%20Reference) (OtherActor :type Actor%20Object%20Reference) (OtherComp :type Primitive%20Component%20Object%20Reference) (OtherBodyIndex :type Integer) (bFromSweep :type Boolean) (SweepResult :type Hit%20Result%20Structure%20%28by%20ref%29))
  (if (== OtherActor (Game|GetPlayerCharacter 0))
    (Variables|Default|SetOverlap true)))

(event OnComponentEndOverlap(Sphere)
  (params (OverlappedComponent :type Primitive%20Component%20Object%20Reference) (OtherActor :type Actor%20Object%20Reference) (OtherComp :type Primitive%20Component%20Object%20Reference) (OtherBodyIndex :type Integer))
  (if (== OtherActor (Game|GetPlayerCharacter 0))
    (Variables|Default|SetOverlap false)))

(event Custom|Activate
  (params (InDirection :type Vector) (InRotation :type Rotator))
  (bind _projectilemovement (Variables|Default|GetProjectileMovement))
  (Variables|/Script/Engine.MovementComponent|SetVelocity _projectilemovement (* InDirection (Variables|/Script/Engine.ProjectileMovementComponent|GetInitialSpeed _projectilemovement)))
  (Components|Activation|Activate _projectilemovement false))

(event EventTick
  (params (DeltaSeconds :type Float%20%28single-precision%29))
  (bind _returnvalue (Game|GetPlayerCharacter 0))
  (bind _sphere (Variables|Default|GetSphere))
  (Utilities|FlowControl|Sequence
    (:then_0
      (if (Variables|Default|GetOverlap)
        (Class|IDamage|Damaged(Message) _returnvalue _returnvalue self (Variables|Default|GetHitData) true)))
    (:then_1
      (Components|Sphere|SetSphereRadius _sphere (Math|Interpolation|FInterpTo (Variables|/Script/Engine.SphereComponent|GetSphereRadius _sphere) (Variables|Default|GetMaxRadius) DeltaSeconds 1.0) true))))

(fn ConstructionScript)