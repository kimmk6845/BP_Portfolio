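; Boss enemy that targets the player through a blackboard key set by overlap spheres and drives the player's boss health bar by distance and damage.
; Attack events cover random melee montages, a dash skill with pass-through collision, a teleport behind the player with boosted damage, and ranged skills scattered around the target.
; Melee damage uses a sphere overlap, also triggered by capsule contact while dashing.
; Niagara trails on listed bones dress the dashes.
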(fn ConstructionScript
  (|CallParentFunction))

(fn SetTarget
  (params (NewTarget :type Character%20Object%20Reference))
  (AI|Components|Blackboard|SetValueasObject (AI|GetBlackboard (AI|GetAIController self)) (Utilities|Name|MakeLiteralName "Target") NewTarget))

(fn GetTarget
  (if (> (Variables|Default|GetHealth) 0.0)
    (return (.AsCharacter (Utilities|Casting|CastToCharacter (AI|Components|Blackboard|GetValueasObject (AI|GetBlackboard (AI|GetAIController self)) (Utilities|Name|MakeLiteralName "Target")))))))

(fn ClearTarget
  (AI|Components|Blackboard|ClearValue (AI|GetBlackboard (AI|GetAIController self)) (Utilities|Name|MakeLiteralName "Target")))

(fn DashEffectStart
  (Effects|SpawnEmitteratLocation "/Game/Effects/P_BossDash.P_BossDash" (Transformation|GetWorldLocation (Variables|Character|GetMesh)))
  (bind _returnvalue (Niagara|SpawnSystemAttached "/Game/ImproveFights_Vfx/Particles/P_Darkness_Dash.P_Darkness_Dash" (Variables|Character|GetMesh) "None" "0, 0, 0" "0, 0, 0" "KeepRelativeOffset" true))
  (Variables|Default|SetDashEffect _returnvalue)
  (for _array_element (Variables|Dash|GetBones_Dash)
    (bind _returnvalue_2 (Niagara|SpawnSystemAttached "/Game/ImproveFights_Vfx/Particles/P_Darkness_DashTrail.P_Darkness_DashTrail" (Variables|Character|GetMesh) (.bone_name _array_element) "0, 0, 0" "0, 0, 0" "KeepRelativeOffset" true))
    (bind _output_get (Variables|Default|SetDashTrailEffect _returnvalue_2))
    (Effects|Components|ParticleSystem|SetFloatParameter _output_get "User.RibbonWidth" (.ribbon_width _array_element))
    (Effects|Components|ParticleSystem|SetFloatParameter _output_get "User.RibbonLenght" (.ribbon_length _array_element))
    (Effects|Components|ParticleSystem|SetFloatParameter _output_get "User.Duration" (Variables|Dash|GetDash_Duration)))
  (Utilities|FlowControl|Sequence
    (:then_0
      (Utilities|IsValid (Variables|Default|GetDashTrailEffect)
        (:Is%20Valid
          (Components|Activation|Deactivate (Variables|Default|GetDashTrailEffect)))))))

(fn DashParticleStart
  (Effects|SpawnEmitteratLocation "/Game/Effects/P_BossDash.P_BossDash" (Transformation|GetWorldLocation (Variables|Character|GetMesh))))

(event EventBeginPlay
  (|CallParentFunction)
  (Variables|Default|SetDamageRadius 1.3e+02))

(event EventTick
  (params (DeltaSeconds :type Float%20%28single-precision%29))
  (bind _as_bp_player (Variables|Default|GetAs%20BP%20Player))
  (bind _playerwidget (Variables|/Game/Player/BP_Player.BP_Player_C|GetPlayerWidget _as_bp_player))
  (bind _wb_bosshealthbar (Variables|/Game/Widgets/WB_PlayerWidget.WB_PlayerWidget_C|GetWB_BossHealthBar _playerwidget))
  (|CallParentFunction DeltaSeconds)
  (Utilities|FlowControl|Sequence
    (:then_0
      (if (and (<= (Transformation|GetDistanceTo self (Variables|Default|GetAs%20BP%20Player)) 2.5e+03) (> (Variables|Default|GetHealth) 0.0))
        (Widget|SetVisibility _wb_bosshealthbar "Visible")
        (else
          (Widget|SetVisibility _wb_bosshealthbar "Hidden"))))
    (:then_1
      (if (<= (Variables|Default|GetHealth) 0.0)
        (Variables|Default|SetDie true)))))

(event OnComponentEndOverlap(EndTargetSphere)
  (params (OverlappedComponent :type Primitive%20Component%20Object%20Reference) (OtherActor :type Actor%20Object%20Reference) (OtherComp :type Primitive%20Component%20Object%20Reference) (OtherBodyIndex :type Integer))
  (if (and (== OtherActor (CallFunction|GetTarget)) (not (Variables|Default|GetDie)))
    (CallFunction|ClearTarget)))

(event OnComponentBeginOverlap(CapsuleComponent)
  (params (OverlappedComponent :type Primitive%20Component%20Object%20Reference) (OtherActor :type Actor%20Object%20Reference) (OtherComp :type Primitive%20Component%20Object%20Reference) (OtherBodyIndex :type Integer) (bFromSweep :type Boolean) (SweepResult :type Hit%20Result%20Structure%20%28by%20ref%29))
  (if (and (== OtherActor (Game|GetPlayerCharacter 0)) (Variables|ShortMeleeAttack|GetDashAttack))
    (CallFunction|DoDamage)))

(event OnComponentBeginOverlap(OnTargetSphere)
  (params (OverlappedComponent :type Primitive%20Component%20Object%20Reference) (OtherActor :type Actor%20Object%20Reference) (OtherComp :type Primitive%20Component%20Object%20Reference) (OtherBodyIndex :type Integer) (bFromSweep :type Boolean) (SweepResult :type Hit%20Result%20Structure%20%28by%20ref%29))
  (if (and (== OtherActor (Game|GetPlayerCharacter 0)) (not (Variables|Default|GetDie)))
    (bind _asbp_player (Utilities|Casting|CastToBP_Player OtherActor))
    (CallFunction|SetTarget _asbp_player)))

(event Custom|ATK01
  (params (Target :type Character%20Object%20Reference))
  (if (not (Variables|Default|GetDie))
    (Utilities|FlowControl|Sequence
      (:then_0
        (Utilities|IsValid Target
          (:Is%20Valid
            (Transformation|SetActorRotation (Math|Rotator|MakeRotator 0.0 0.0 (.yaw (Math|Rotator|FindLookatRotation (Transformation|GetActorLocation) (Transformation|GetActorLocation Target))))))))
      (:then_1
        (Animation|PlayAnimMontage (Utilities|Array|Get(acopy) (Variables|Default|GetAttackMontages) (Math|Random|RandomIntegerinRange 0 3)) 1.0 "None")))))

(event Custom|ATK01_2
  (if (not (AI|Components|NavMovement|IsFalling (Variables|Character|GetCharacterMovement)))
    (Variables|Default|SetBoss_DoingSkill true)
    (CallFunction|DashEffectStart)
    (Animation|PlayAnimMontage "/Game/Enemies/Boss/Montages/Boss_ShortMeleeSkill_Montage.Boss_ShortMeleeSkill_Montage" 1.0 "None")))

(event Custom|DoingAttack
  (bind _returnvalue (Transformation|GetActorForwardVector))
  (bind _returnvalue_2 (Math|Conversions|RotationFromXVector _returnvalue))
  (bind _returnvalue_3 (Math|Rotator|MakeRotator 0.0 0.0 (.yaw _returnvalue_2)))
  (bind _returnvalue_4 (Math|Vector|GetForwardVector _returnvalue_3))
  (CallFunction|DashEffectStart)
  (Collision|SetCollisionProfileName (Variables|Default|GetCapsuleComponent) "NoPawn" true :!class /Script/Engine.PrimitiveComponent)
  (Variables|ShortMeleeAttack|SetDashAttack true)
  (Variables|Default|SetBoss_DoingSkill false)
  (bind _returnvalue_5 (Game|SpawnActorfromClass "/Game/Enemies/Boss/BP_BossShortMeleeSkill.BP_BossShortMeleeSkill_C" (Math|Transform|MakeTransform (Transformation|GetActorLocation) (Math|Conversions|RotationFromXVector _returnvalue_4)) "AlwaysSpawn" self 0))
  (Utilities|IsValid _returnvalue_5
    (:Is%20Valid
      (Default|Activate _returnvalue_5 _returnvalue_4 "0, 0, 0")
      (CallFunction|DashParticleStart))))

(event Custom|End_ATK01_2
  (Collision|SetCollisionProfileName (Variables|Default|GetCapsuleComponent) "Pawn" true :!class /Script/Engine.PrimitiveComponent)
  (Variables|ShortMeleeAttack|SetDashAttack false))

(event Custom|DoDamage
  (bind (_outactors _returnvalue) (Collision|SphereOverlapActors (Transformation|GetWorldLocation (Variables|Default|GetDoDamageArrow)) (Variables|Default|GetDamageRadius) (Utilities|Array|MakeArray "ObjectTypeQuery3") 0 (Utilities|Array|MakeArray self)))
  (if _returnvalue
    (for _array_element _outactors
      (bind _asbp_player (Utilities|Casting|CastToBP_Player _array_element))
      (Utilities|IsValid _asbp_player
        (:Is%20Valid
          (Game|Damage|ApplyDamage _asbp_player (Variables|Default|GetDamage) (Pawn|GetController) self))))))

(event EventDamaged
  (params (Attacker :type Character%20Object%20Reference) (Causer :type Actor%20Object%20Reference) (HitData :type F%20Hit%20Data%20Structure) (DisableAvoid :type Boolean))
  (|CallParentFunction Attacker Causer HitData false)
  (Default|UpdateBossHealth (Variables|/Game/Player/BP_Player.BP_Player_C|GetPlayerWidget (Variables|Default|GetAs%20BP%20Player)) (Variables|Default|GetHealth) (Variables|Default|GetMaxHealth)))

(event Game|Damage|EventAnyDamage
  (params (Damage :type Float%20%28single-precision%29) (DamageType :type Damage%20Type%20Object%20Reference) (InstigatedBy :type Controller%20Object%20Reference) (DamageCauser :type Actor%20Object%20Reference))
  (|CallParentFunction Damage DamageType InstigatedBy DamageCauser)
  (Default|UpdateBossHealth (Variables|/Game/Player/BP_Player.BP_Player_C|GetPlayerWidget (Variables|Default|GetAs%20BP%20Player)) (Variables|Default|GetHealth) (Variables|Default|GetMaxHealth)))

(event Custom|ATK03
  (bind _target (CallFunction|GetTarget))
  (bind _returnvalue (Transformation|GetActorLocation _target))
  (if (not (Variables|Default|GetDie))
    (Utilities|FlowControl|Sequence
      (:then_0
        (Transformation|SetActorRotation (Math|Rotator|FindLookatRotation (Transformation|GetActorLocation) (Transformation|GetActorLocation (CallFunction|GetTarget))))
        (Animation|PlayAnimMontage "/Game/Enemies/Boss/Montages/SK_Mannequin_Mage_Skill03_Montage.SK_Mannequin_Mage_Skill03_Montage" 1.0 "None"))
      (:then_1
        (while (<= (Utilities|Array|Length (Variables|Default|GetSkillSpawnLocation)) 4)
          (Utilities|Array|Add (Variables|Default|GetSkillSpawnLocation) (Math|Vector|MakeVector (+ (Math|Random|RandomFloatinRange -1e+03 1e+03) (.x _returnvalue)) (+ (Math|Random|RandomFloatinRange -1e+03 1e+03) (.y _returnvalue)) (- (.z _returnvalue) 88.0))))
        (for _array_element (Variables|Default|GetSkillSpawnLocation)
          (Game|SpawnActorfromClass "/Game/Enemies/Boss/BP_BossRangeSkill.BP_BossRangeSkill_C" (Math|Transform|MakeTransform _array_element "0, 0, 0" "1,1,1") "Undefined" 0 0))
        (Utilities|Array|Clear (Variables|Default|GetSkillSpawnLocation))))))

(event Custom|ATK02
  (params (Target :type Character%20Object%20Reference))
  (bind _returnvalue (Game|GetPlayerCharacter 0))
  (if (not (Variables|Default|GetDie))
    (CallFunction|DashEffectStart)
    (Transformation|SetActorLocation (+ (Transformation|GetActorLocation _returnvalue) (* (Transformation|GetActorForwardVector _returnvalue) -1e+02)) false false)
    (CallFunction|DashParticleStart)
    (Animation|PlayAnimMontage (Utilities|Array|Get(acopy) (Variables|Default|GetBackAttackMontages) (Math|Random|RandomIntegerinRange 0 3)) 1.0 "None")
    (Variables|Default|SetDamageRadius 4e+02)
    (Variables|Default|SetDamage 5e+01)))

(event Custom|End_ATK02
  (bind _returnvalue (Transformation|GetActorLocation))
  (bind _returnvalue_2 (- _returnvalue "0, 0,120.000000"))
  (Variables|Default|SetDamageRadius 1.3e+02)
  (Variables|Default|SetDamage 3e+01)
  (Niagara|SpawnSystematLocation "/Game/Effects/NS_Warrior_EarthCrack.NS_Warrior_EarthCrack" _returnvalue_2)
  (Audio|PlaySoundatLocation "/Game/Sounds/Boss_DashSkill.Boss_DashSkill" _returnvalue_2 "0, 0, 0" 1.0 1.0 0.0 0 0 0))