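; Enemy character that takes hits from the player or rival-group enemies, guards, and dies.
; Damage events drive StateComponent, whose Hitted state either blocks and staggers the attacker (skills break guard) or applies damage.
; Hits trigger effects, camera shake, red flash, knockback and hit-stop via per-actor time dilation.
; Bosses mid-skill take damage without flinching, and radial damage has its own guard-breaking knockback path.
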(event Custom|Dead
  ;[1 1 1] Dead
  (Default|SetDeadMode (Variables|Default|GetStateComponent))
  (Collision|SetCollisionEnabled (Variables|Collision|GetCapsuleComponent) "NoCollision")
  (Animation|PlayAnimMontage "/Game/Enemies/Boss/Montages/Katana_Blade_Damage_Die_Montage.Katana_Blade_Damage_Die_Montage" 1.0 "None"))

(event Custom|End_Dead
  ;[1 1 1] Dead
  (Default|DetachWeapon (Variables|Default|GetWeaponComponent))
  (Actor|DestroyActor))

(event Custom|OnStateTypeChanged
  (params (InPrevType :type EStateType%20Enum :default "NewEnumerator0") (InNewType :type EStateType%20Enum :default "NewEnumerator0"))
  (switch Utilities|FlowControl|Switch|SwitchonEStateType InNewType
    (:NewEnumerator5
      (CallFunction|Hitted))
    (:NewEnumerator8
      (CallFunction|Blocked))))

(event Custom|SkillHitted
  (|SetDamage2 (.Damage (Utilities|Struct|BreakFHitData (Variables|Hitted|GetHitData)))
    (:Dead
      (CallFunction|Dead))))

(event Custom|Blocked
  (bind _statuscomponent (Variables|Default|GetStatusComponent))
  ;[1 1 1] Blocked
  (Default|BackupControlRotation _statuscomponent)
  (Default|DisableControlRotation _statuscomponent)
  (Animation|PlayAnimMontage "/Game/Enemies/Montages/Common/Block_Montage.Block_Montage" 1.0 "None"))

(event Custom|End_Blocked
  ;[1 1 1] Blocked
  (Default|RestoreControlRotation (Variables|Default|GetStatusComponent))
  (Default|SetIdleMode (Variables|Default|GetStateComponent)))

(event EventDamaged
  (params (Attacker :type Character%20Object%20Reference) (Causer :type Actor%20Object%20Reference) (HitData :type F%20Hit%20Data%20Structure) (DisableAvoid :type Boolean))
  (bind _output_get (Variables|Hitted|SetAttacker Attacker))
  (bind _asbp_enemy_ai (Utilities|Casting|CastToBP_Enemy_AI _output_get)
    (:then
      (Utilities|IsValid _asbp_enemy_ai
        (:Is%20Valid
          (if (not (Utilities|Enum|Equal(Enum) (Variables|BP_Enemy_C|GetGroup _asbp_enemy_ai) (Variables|Group|GetGroup)))
            (Variables|Hitted|SetCauser Causer :!label _label)
            (Variables|Hitted|SetHitData HitData)
            (if (> (Variables|Default|GetHealth) 0.0)
              (if (Variables|Default|GetBoss_DoingSkill)
                (CallFunction|SkillHitted)
                (|BossHitEffect)
                (else
                  (Default|SetHittedMode (Variables|Default|GetStateComponent)))))))))
    (:CastFailed
      (goto _label))))

(event Game|Damage|EventAnyDamage
  (params (Damage :type Float%20%28single-precision%29) (DamageType :type Damage%20Type%20Object%20Reference) (InstigatedBy :type Controller%20Object%20Reference) (DamageCauser :type Actor%20Object%20Reference))
  ;[1 1 1] Radial Damage Hitted
  (bind _ascharacter (Utilities|Casting|CastToCharacter (Components|GetOwner DamageCauser)))
  (Utilities|IsValid _ascharacter
    (:Is%20Valid
      (Variables|Hitted|SetAttacker _ascharacter)
      (if (> (Variables|Default|GetHealth) 0.0)
        (|RadialDamageHitted Damage)))))

(event EventTick
  (params (DeltaSeconds :type Float%20%28single-precision%29))
  (bind _returnvalue (Transformation|GetActorLocation))
  (Utilities|FlowControl|Sequence
    (:then_0
      (if (Default|IsActionMode (Variables|Default|GetStateComponent))
        (Variables|Guard|SetGuarding false)))
    (:then_1
      ;[1 0 0.2795] 임시, 적이 공격중이면 튕겨나갈때도 있음
      (bind _asbp_player (Utilities|Casting|CastToBP_Player (Variables|Hitted|GetAttacker)))
      (Utilities|IsValid _asbp_player
        (:Is%20Valid
          (if (Math|Boolean|ANDBoolean (Variables|/Game/Player/BP_Player.BP_Player_C|GetT_Skilling _asbp_player) (Default|IsHittedMode (Variables|Default|GetStateComponent)) (AI|Components|NavMovement|IsFalling (Variables|Character|GetCharacterMovement)))
            (Transformation|SetActorLocation (Math|Vector|MakeVector (.x _returnvalue) (.y _returnvalue) (.z (Transformation|GetWorldLocation (Variables|/Game/Player/BP_Player.BP_Player_C|GetSceneAirAction _asbp_player)))) false false)))))))

(event EventBeginPlay
  (Utilities|FlowControl|Sequence
    (:then_0
      (for _array_element (Rendering|Material|GetMaterials (Variables|Character|GetMesh))
        (bind _returnvalue (Rendering|Material|CreateDynamicMaterialInstance _array_element "None" "None" :!class /Script/Engine.KismetMaterialLibrary))
        (bind _returnvalue_2 (Utilities|Array|Add (Variables|Default|GetMaterials) _returnvalue))
        (Rendering|Material|SetMaterial (Variables|Character|GetMesh) _returnvalue_2 _returnvalue)
        (for _array_element_2 (Variables|Default|GetMaterials)
          (Rendering|Material|SetVectorParameterValue _array_element_2 "BodyColor" (Variables|Material|GetColor) :!class /Script/Engine.MaterialInstanceDynamic)
          (bind _asbp_player (Utilities|Casting|CastToBP_Player (Game|GetPlayerCharacter 0)))
          (Variables|Default|SetAs%20BP%20Player _asbp_player))))
    (:then_1
      (EventDispatchers|AssignOnStateTypeChanged (Variables|Default|GetStateComponent) (delegate Custom|OnStateTypeChanged)))
    (:then_2
      (Variables|Default|SetHealth (Variables|Default|GetMaxHealth)))
    (:then_3
      (bind _returnvalue_3 (Niagara|SpawnSystemAttached "/Game/Effects/NS_TSkillHelper.NS_TSkillHelper" (Variables|Character|GetMesh) "None" "0, 0,130.000000" "0, 0, 0" "KeepRelativeOffset" false))
      (bind _output_get (Variables|Default|SetOneHand_SkillHelper _returnvalue_3))
      (Rendering|SetVisibility _output_get false false))))

(fn ConstructionScript)

(fn OnRendering
  (Default|OnRendering (Variables|Default|GetWeaponComponent)))

(fn OffRendering
  (Default|OffRendering (Variables|Default|GetWeaponComponent)))

(event Custom|Hitted
  (bind _attacker (Variables|Hitted|GetAttacker))
  (bind _returnvalue (Actor|GetComponentbyClass _attacker "/Game/Components/StateComponent.StateComponent_C"))
  (if (Variables|Guard|GetGuarding)
    (Utilities|IsValid _returnvalue
      (:Is%20Valid
        (if (Default|IsSkillMode _returnvalue)
          ;[1 1 1] 스킬 Hit = 가드 파괴
          (CallFunction|GuardReleased)
          (|SetDamage (.Damage (Utilities|Struct|BreakFHitData (Variables|Hitted|GetHitData))) :!label _label
            (:Dead
              (CallFunction|Dead))
            (:Hitted
              (Game|Damage|ApplyDamage)))
          (else
            (|Blocking :!label _label_2))))
      (:Is%20Not%20Valid
        (goto _label_2)))
    (else
      (goto _label))))

(event Custom|RestoreTimeDelation
  (bind _delationactors (Variables|Default|GetDelationActors))
  (for _array_element _delationactors
    (Variables|/Script/Engine.Actor|SetCustomTimeDilation _array_element 1.0))
  (Utilities|Array|Clear _delationactors))

(event Custom|GuardPressed
  (if (Default|IsIdleMode (Variables|Default|GetStateComponent))
    (Animation|PlayAnimMontage (.guardanim (Variables|/Game/Components/WeaponComponent.WeaponComponent_C|GetGuardAnimData (Variables|Default|GetWeaponComponent))) 1.0 "None")
    (Default|EndDoAction (Variables|Default|GetWeaponComponent))
    (Variables|Guard|SetGuarding true)))

(event Custom|GuardReleased
  (Animation|StopAnimMontage (.guardanim (Variables|/Game/Components/WeaponComponent.WeaponComponent_C|GetGuardAnimData (Variables|Default|GetWeaponComponent))))
  (Variables|Guard|SetGuarding false)
  (Default|SetIdleMode (Variables|Default|GetStateComponent)))