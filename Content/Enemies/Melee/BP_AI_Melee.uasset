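; BP_AI_Melee is the melee enemy AI Blueprint, extending a parent class that supplies its core behavior.
; It adds a stun indicator: the PStun component is hidden at BeginPlay, shown on Begin_Stun and hidden again on End_Stun.
; The construction script only calls the parent implementation.
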(event Custom|End_Stun
  (Rendering|SetVisibility (Variables|Default|GetP_Stun) false false))

(event Custom|Begin_Stun
  (Rendering|SetVisibility (Variables|Default|GetP_Stun) true false))

(event EventBeginPlay
  (|CallParentFunction)
  (Rendering|SetVisibility (Variables|Default|GetP_Stun) false false))

(fn ConstructionScript
  (|CallParentFunction))